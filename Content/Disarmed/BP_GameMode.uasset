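; Game mode for Disarmed that runs the match countdown and handles game over.
; Tick drives a state machine from counting to game over, showing the game-over widget, playing the victory sound and firing the game-over call, then enabling input after a short delay.
; Getters expose time remaining and state.
; On BeginPlay, a zero player count in the game instance signals an editor play session and adds a player for two-player debugging.
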(event EventBeginPlay
  ;[1 1 1] Debug with two players
  (|DidWeStartInPieFromTheEditor)
  (Class|GameplayStatics|CreatePlayer -1))

(event EventTick
  (params (DeltaSeconds :type Float%20%28single-precision%29))
  (switch Utilities|FlowControl|Switch|SwitchonEGameModeState (Variables|Default|GetState)
    (:NewEnumerator0
      (bind _output_get (Variables|Default|SetSecondsRemaining (- (Variables|Default|GetSecondsRemaining) DeltaSeconds)))
      (if (<= _output_get 0.0)
        (Variables|Default|SetState "NewEnumerator1")
        (bind _returnvalue (UserInterface|CreateWidget "/Game/Disarmed/UI/WBP_GameOver.WBP_GameOver_C" (Game|GetPlayerController 0)))
        (UserInterface|Viewport|AddtoViewport _returnvalue 0)
        (Audio|PlaySound2D "/Game/Disarmed/SFX/A_Victory.A_Victory" 1.0 1.0 0.0 0 0)
        (Default|CallOnGameOver)
        (Utilities|FlowControl|Delay 2.0)
        (Variables|Default|SetState "NewEnumerator2")))))

(fn ConstructionScript)

(fn GetSecondsRemaining
  (return (Variables|Default|GetSecondsRemaining)))

(fn IsGameinProgress
  (return (Utilities|Enum|Equal(Enum) (Variables|Default|GetState) "NewEnumerator0")))

(fn IsGameOverInputEnabled
  (return (Utilities|Enum|Equal(Enum) (Variables|Default|GetState) "NewEnumerator2")))