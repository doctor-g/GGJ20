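; BP_Pickup is a world pickup that gives an overlapping BP_Robot a new arm.
; On sphere overlap, it grants the arm if the robot has none or if CanPickupArmReplacement allows swapping the current one.
; It spawns an actor of ArmClass, passes it to the robot's SetArm, plays a 2D pickup sound and destroys itself.
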(event OnComponentBeginOverlap(Sphere)
  (params (OverlappedComponent :type Primitive%20Component%20Object%20Reference) (OtherActor :type Actor%20Object%20Reference) (OtherComp :type Primitive%20Component%20Object%20Reference) (OtherBodyIndex :type Integer) (bFromSweep :type Boolean) (SweepResult :type Hit%20Result%20Structure%20%28by%20ref%29))
  (bind _asbp_robot (Utilities|Casting|CastToBP_Robot OtherActor))
  (bind _hasarm (Default|HasArm _asbp_robot))
  (if _hasarm
    (if (Default|CanPickupArmReplacement _asbp_robot)
      (bind _returnvalue (Game|SpawnActorfromClass (Variables|Default|GetArmClass) (Math|Transform|MakeTransform "0, 0, 0") "Undefined" 0 0 :!label _label))
      (Default|SetArm _asbp_robot _returnvalue)
      (Audio|PlaySound2D "/Game/Disarmed/SFX/A_Pickup.A_Pickup" 1.0 1.0 0.0 0 0)
      (Actor|DestroyActor))
    (else
      (goto _label))))

(event EventBeginPlay)

(event Collision|EventActorBeginOverlap
  (params (OtherActor :type Actor%20Object%20Reference)))

(event EventTick
  (params (DeltaSeconds :type Float%20%28single-precision%29)))

(fn ConstructionScript)