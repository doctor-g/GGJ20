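; Robot harpoon arm weapon that fires a limited supply of harpoons.
; On shoot release it spawns a BP_Harpoon at its own transform, launches it along local forward, decrements the count and updates its sprite to match.
; When empty, it plays a sound instead of firing.
; It overrides CanPickupReplacement to allow a replacement pickup whenever fewer than three harpoons remain.
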(event EventTick
  (params (DeltaSeconds :type Float%20%28single-precision%29)))

(event EventOnShootReleased
  (if (> (Variables|Default|GetHarpoonsRemaining) 0)
    (bind _returnvalue (Game|SpawnActorfromClass "/Game/Disarmed/Robot/Weapons/Harpoon/BP_Harpoon.BP_Harpoon_C" (Transformation|GetActorTransform) "AlwaysSpawn" (Components|GetOwner) 0))
    (Game|Components|ProjectileMovement|SetVelocityinLocalSpace (Variables|/Game/Disarmed/Robot/Weapons/Harpoon/BP_Harpoon.BP_Harpoon_C|GetProjectileMovement _returnvalue) "2000.000000, 0, 0")
    (bind _result (Math|Integer|DecrementInt (Variables|Default|GetHarpoonsRemaining))
      (:%20%20
        (Rendering|Components|Sprite|SetSprite (Variables|Default|GetPaperSprite) (Utilities|Array|Get(acopy) (Variables|Default|GetSprites) _result))))
    (else
      (Audio|PlaySound2D "/Game/Disarmed/SFX/A_Shoot.A_Shoot" 1.0 1.0 0.0 0 0))))

(event EventBeginPlay
  (Input|EnableInput 0))

(fn ConstructionScript
  (|CallParentFunction))

(fn CanPickupReplacement
  (return (< (Variables|Default|GetHarpoonsRemaining) 3)))