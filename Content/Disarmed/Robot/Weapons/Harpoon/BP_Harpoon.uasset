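; BP_Harpoon is a 2D harpoon weapon actor that damages robots it touches.
; Its Paper2D sprite overlap ignores the owning actor and calls DamageRobot on any other BP_Robot, passing the owner robot, then destroys the harpoon.
; It also destroys itself on overlapping WorldStatic components, while other overlaps are ignored.
; Movement is not handled in these graphs.
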(event OnComponentBeginOverlap(PaperSprite)
  (params (OverlappedComponent :type Primitive%20Component%20Object%20Reference) (OtherActor :type Actor%20Object%20Reference) (OtherComp :type Primitive%20Component%20Object%20Reference) (OtherBodyIndex :type Integer) (bFromSweep :type Boolean) (SweepResult :type Hit%20Result%20Structure%20%28by%20ref%29))
  (if (not (== OtherActor (Components|GetOwner)))
    (bind _asbp_robot (Utilities|Casting|CastToBP_Robot OtherActor)
      (:then
        (Default|DamageRobot _asbp_robot (.AsBP%20Robot (Utilities|Casting|CastToBP_Robot (Components|GetOwner))))
        (Actor|DestroyActor))
      (:CastFailed
        ;[1 1 1] Destroy me if I run into a world static object
        (if (Utilities|Enum|Equal(Enum) (Collision|GetCollisionObjectType OtherComp) "ECC_WorldStatic")
          (Actor|DestroyActor))))))

(event EventBeginPlay)

(event Collision|EventActorBeginOverlap
  (params (OtherActor :type Actor%20Object%20Reference)))

(event EventTick
  (params (DeltaSeconds :type Float%20%28single-precision%29)))

(fn ConstructionScript)