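; Player-controlled Paper2D robot for the Disarmed arena game, tinted per player, with a swappable arm as its weapon.
; Input drives walking, jumping, arm aiming and shooting (which halts walking), while Tick updates flipbooks and facing.
; The first hit destroys the arm; an armless hit kills, updates kill/death tallies, and respawns at the start transform after the death animation.
; GameMode-checking macros gate most gameplay input and the game-over rematch/quit actions.
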(event Custom|DamageRobot
  (params (Attacker :type BP%20Robot%20Object%20Reference))
  (bind _sprite (Variables|Default|GetSprite))
  ;[1 1 1] DamageRobot
  (Utilities|GameinProgress
    (:In%20Progress
      (if (not (Variables|Default|GetIsDying))
        (bind _arm (Variables|Default|GetArm)
          (:then
            (Game|SpawnActorfromClass "/Game/Disarmed/Robot/Weapons/Explosion/BP_Explosion.BP_Explosion_C" (Transformation|GetActorTransform _arm) "Undefined" 0 0)
            (Actor|DestroyActor _arm)
            (Variables|Default|SetArm 0)
            (Audio|PlaySound2D "/Game/Disarmed/SFX/A_Armexplosion.A_Armexplosion" 1.0 1.0 0.0 0 0))
          (:else
            (Variables|Default|SetIsDying true)
            (Sprite|SetFlipbook _sprite "/Game/Disarmed/Robot/Death/PFB_Death.PFB_Death")
            (Components|Timeline|SetLooping _sprite false)
            (EventDispatchers|BindEventtoOnFinishedPlaying _sprite (delegate Custom|OnDeathAnimationComplete))
            (Audio|PlaySound2D "/Game/Disarmed/SFX/A_Death.A_Death" 1.0 1.0 0.0 0 0)
            (Math|Integer|IncrementInt (Variables|Default|GetDeaths)
              (:%20%20
                (CallFunction|AddKill Attacker)))))))))

(event Custom|UpdateAnimation
  ;[1 1 1] Handle Animation
  (if (not (Variables|Default|GetIsDying))
    (Sprite|SetFlipbook (Variables|Default|GetSprite) (select (> (Math|Vector|VectorLength (Transformation|GetVelocity)) 0.0) "/Game/Disarmed/Robot/PFB_Walk.PFB_Walk" "/Game/Disarmed/Robot/PFB_Idle.PFB_Idle"))))

(event Custom|OnDeathAnimationComplete
  (bind _sprite (Variables|Default|GetSprite))
  ;[1 1 1] DamageRobot
  (Transformation|SetActorTransform (Variables|Default|GetInitialTransform) false true)
  (Variables|Default|SetIsDying false)
  (Components|Timeline|SetLooping _sprite true)
  (Audio|Components|Audio|Play _sprite) ; Have to call this to prevent animation lockup
  (EventDispatchers|UnbindEventfromOnFinishedPlaying _sprite (delegate Custom|OnDeathAnimationComplete)))

(event Custom|OnGameOver
  ;[1 1 1] When the game is over, unpossess and stop ticking
  (Actor|Tick|SetActorTickEnabled false))

(event EventPossessed
  (params (NewController :type Controller%20Object%20Reference))
  ;[1 1 1] Event Possessed: Set the robot color
  (bind _asplayer_controller (Utilities|Casting|CastToPlayerController NewController))
  (Rendering|Material|SetMaterial (Variables|Default|GetSprite) 0 (CallFunction|GetPlayerColor (Class|GameplayStatics|GetPlayerControllerID _asplayer_controller))))

(event EventBeginPlay
  ;[1 1 1] BeginPlay: Record my spawn point
  (Variables|Default|SetInitialTransform (Transformation|GetActorTransform))
  (bind _asbp_game_mode (Utilities|Casting|CastToBP_GameMode (Game|GetGameMode)))
  (EventDispatchers|BindEventtoOnGameOver _asbp_game_mode (delegate Custom|OnGameOver)))

(event EventTick
  (params (DeltaSeconds :type Float%20%28single-precision%29))
  (bind _armslot (Variables|Default|GetArmSlot))
  (bind _relativelocation (Variables|/Script/Engine.SceneComponent|GetRelativeLocation _armslot))
  (bind _relativelocation_2 (Variables|/Script/Engine.SceneComponent|GetRelativeLocation _armslot))
  ;[1 1 1] Tick - Updates animation
  (CallFunction|UpdateAnimation)
  (Math|Float|CompareFloat (.X (Math|Vector|BreakVector (Variables|/Script/Engine.MovementComponent|GetVelocity (Pawn|GetMovementComponent)))) 0.0
    (:>
      (Pawn|SetControlRotation (Pawn|GetController) (Math|Rotator|MakeRotator 0.0 0.0 0.0) :!label _label)
      (Transformation|SetRelativeLocation _armslot (Math|Vector|MakeVector (.x _relativelocation_2) 1.0 (.z _relativelocation_2)) false false))
    (:==
      (if (Variables|Default|GetIsMovingRight)
        (goto _label)
        (else
          (Pawn|SetControlRotation (Pawn|GetController) (Math|Rotator|MakeRotator 0.0 0.0 1.8e+02) :!label _label_2)
          (Transformation|SetRelativeLocation _armslot (Math|Vector|MakeVector (.x _relativelocation) -1.0 (.z _relativelocation)) false false))))
    (:<
      (goto _label_2))))

(event Input|ActionEvents|InputActionShoot
  (params (Key :type Key%20Structure :default "None"))
  ;[1 1 1] Shoot
  (:Pressed
    (Utilities|GameinProgress
      (:In%20Progress
        (if (not (Variables|Default|GetIsDying))
          (bind _arm (Variables|Default|GetArm)
            (:then
              (Default|OnShootPressed _arm)
              (Variables|Default|SetIsShooting true))
            (:else))))))
  (:Released
    (Utilities|GameinProgress
      (:In%20Progress
        (Variables|Default|SetIsShooting false)
        (bind _arm_2 (Variables|Default|GetArm)
          (:then
            (Default|OnShootReleased _arm_2))
          (:else))))))

(event Input|ActionEvents|InputActionRematch
  (params (Key :type Key%20Structure :default "None"))
  (:Pressed
    (Utilities|GameOverwithInputEnabled
      (:out
        (Game|OpenLevel(byName) "/Game/Disarmed/Maps/Arena")))))

(event Input|ActionEvents|InputActionQuitGame
  (params (Key :type Key%20Structure :default "None"))
  (:Pressed
    (Utilities|GameOverwithInputEnabled
      (:out
        (Game|QuitGame 0 "Quit" false)))))

(event Input|ActionEvents|InputActionJump
  (params (Key :type Key%20Structure :default "None"))
  ;[1 1 1] Handle Jump
  (:Pressed
    (if (not (Variables|Default|GetIsDying))
      (Character|Jump)))
  (:Released
    (Character|StopJumping)))

(event Input|AxisEvents|InputAxisAimUp
  (params (AxisValue :type Float%20%28single-precision%29))
  ;[1 1 1] Aim
  (Utilities|GameinProgress
    (:In%20Progress
      (Transformation|SetRelativeRotation (Variables|Default|GetArmSlot) (Math|Rotator|MakeRotator 0.0 (Math|Float|Lerp 0.0 9e+01 AxisValue) 0.0) false false))))

(event Input|AxisEvents|InputAxisMoveRight
  (params (AxisValue :type Float%20%28single-precision%29))
  ;[1 1 1] Handle movement
  (if (not (Variables|Default|GetIsDying))
    (Utilities|GameinProgress
      (:In%20Progress
        (if (> AxisValue 0.0)
          (Variables|Default|SetIsMovingRight true)
          (elif (< AxisValue 0.0)
            (Variables|Default|SetIsMovingRight false)))
        (Pawn|Input|AddMovementInput "1.000000, 0, 0" (select (Variables|Default|GetIsShooting) 0.0 AxisValue) false)))))

(event Input|TouchEvents|InputTouch
  (params (Location :type Vector) (FingerIndex :type ETouchIndex%20Enum))
  ;[1 1 1] Handle Jump
  (:Pressed
    (if (not (Variables|Default|GetIsDying))
      (Character|Jump)))
  (:Released
    (Character|StopJumping)))

(fn ConstructionScript)

(fn SetArm
  (params (Arm :type BP%20Arm%20Object%20Reference))
  ;[1 1 1] If we already had an arm, destroy it
  (bind _arm (Variables|Default|GetArm)
    (:then
      (Actor|DestroyActor _arm))
    (:else
      _))
  (bind _output_get (Variables|Default|SetArm Arm))
  (Actor|SetOwner _output_get self)
  (Transformation|AttachComponentToComponent _output_get (Variables|Default|GetArmSlot) "None" "SnapToTarget" "SnapToTarget" "KeepRelative" true))

(fn HasArm
  (return (Utilities|IsValid (Variables|Default|GetArm))))

(fn AddKill
  (Math|Integer|IncrementInt (Variables|Default|GetKills)))

(fn CanPickupArmReplacement
  (bind _arm (Variables|Default|GetArm)
    (:then
      (bind _canpickup (Default|CanPickupReplacement _arm))
      (return _canpickup))
    (:else
      (return true))))